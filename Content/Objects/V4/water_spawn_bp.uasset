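; VR water spawner actor that produces water when touched by a BP_MotionController.
; Each such overlap spawns a Water_bp slightly above the static mesh, copying its rotation and scale, and plays the Water sound there.
; The construction script shrinks and flattens the mesh.
; A Break Table function, not called within this Blueprint, swaps the actor for four Tablepeg_bp and one Tabletop_bp actors.
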(event Collision|EventActorBeginOverlap
  (params (OtherActor :type Actor%20Object%20Reference))
  (bind _staticmeshcomponent (Variables|Debug|GetStaticMeshComponent))
  (bind _returnvalue (Transformation|GetWorldTransform _staticmeshcomponent))
  (bind (_location _rotation _scale) (Math|Transform|BreakTransform _returnvalue))
  (bind (_x _y _z) (Math|Vector|BreakVector _location))
  (if (== (Utilities|GetClass OtherActor) "/Game/VirtualRealityBP/Blueprints/BP_MotionController.BP_MotionController_C")
    (Game|SpawnActorfromClass "/Game/Objects/V4/water_bp.water_bp_C" (Math|Transform|MakeTransform (Math|Vector|MakeVector _x _y (+ _z 3e+01)) _rotation _scale) "Undefined" 0 0)
    (Audio|PlaySoundatLocation "/Game/Audio/water.water" _location)))

(fn ConstructionScript
  (Transformation|SetWorldScale3D (Variables|Debug|GetStaticMeshComponent) "0.200000,0.200000,0.100000"))

(fn BreakTable
  (bind _staticmeshcomponent (Variables|Debug|GetStaticMeshComponent))
  (bind _returnvalue (Transformation|GetWorldLocation _staticmeshcomponent))
  (bind _returnvalue_2 (Transformation|GetWorldScale _staticmeshcomponent))
  (bind _returnvalue_3 (Math|Transform|MakeTransform _returnvalue "0, 0, 0" _returnvalue_2))
  (Development|SetHiddeninGame _staticmeshcomponent true false)
  (Game|SpawnActorfromClass "/Game/Objects/tablepeg_bp.tablepeg_bp_C" _returnvalue_3 "Undefined" 0 0)
  (Game|SpawnActorfromClass "/Game/Objects/tablepeg_bp.tablepeg_bp_C" _returnvalue_3 "Undefined" 0 0)
  (Game|SpawnActorfromClass "/Game/Objects/tablepeg_bp.tablepeg_bp_C" _returnvalue_3 "Undefined" 0 0)
  (Game|SpawnActorfromClass "/Game/Objects/tablepeg_bp.tablepeg_bp_C" _returnvalue_3 "Undefined" 0 0)
  (Game|SpawnActorfromClass "/Game/Objects/tabletop_bp.tabletop_bp_C" _returnvalue_3 "Undefined" 0 0)
  (Actor|DestroyActor))