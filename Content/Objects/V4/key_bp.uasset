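; Key actor that can be picked up and dropped by attachment, and opens a jail gate when it touches a keyhole.
; Pickup and Drop toggle mesh physics while attaching or detaching, and the construction script shrinks the mesh.
; Overlapping a component tagged is_key_hole hides every StaticMeshActor tagged jail_bar, without changing collision.
; For each bar, it also sets OpenedGate on character-tagged MotionControllerPawns, printing repeatedly on cast failure.
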(event OnComponentBeginOverlap(StaticMeshComponent)
  (params (OverlappedComponent :type Primitive%20Component%20Object%20Reference) (OtherActor :type Actor%20Object%20Reference) (OtherComp :type Primitive%20Component%20Object%20Reference) (OtherBodyIndex :type Integer) (bFromSweep :type Boolean) (SweepResult :type Hit%20Result%20Structure%20%28by%20ref%29))
  (if (Components|ComponentHasTag OtherComp "is_key_hole")
    (bind _outactors (Actor|GetAllActorsOfClass "/Script/Engine.StaticMeshActor"))
    (for _array_element _outactors
      (if (Actor|ActorHasTag _array_element "jail_bar")
        (Rendering|SetVisibility (Variables|/Script/Engine.StaticMeshActor|GetStaticMeshComponent _array_element) false true)
        (bind _outactors_2 (Actor|GetAllActorswithTag "character"))
        (for _array_element_2 _outactors_2
          (bind _asmotion_controller_pawn (Utilities|Casting|CastToMotionControllerPawn _array_element_2)
            (:then
              (Variables|/Game/VirtualRealityBP/Blueprints/MotionControllerPawn.MotionControllerPawn_C|Setopened_gate _asmotion_controller_pawn true)
              (for _index (range 0 100)
                _))
            (:CastFailed
              (for _index_2 (range 0 100)
                (Development|PrintString "CAST FAILED")))))))))

(event EventBeginPlay)

(event Collision|EventActorBeginOverlap
  (params (OtherActor :type Actor%20Object%20Reference)))

(event EventTick
  (params (DeltaSeconds :type Float%20%28single-precision%29)))

(event EventDrop
  (Physics|SetSimulatePhysics (Variables|Debug|GetStaticMeshComponent) true)
  (Transformation|DetachFromActor "KeepWorld" "KeepWorld" "KeepWorld"))

(event EventPickup
  (params (AttachTo :type Scene%20Component%20Object%20Reference))
  (Physics|SetSimulatePhysics (Variables|Debug|GetStaticMeshComponent) false)
  (Transformation|AttachComponentToComponent (VehicleSound|GetRootComponent) AttachTo "None" "KeepWorld" "KeepWorld" "KeepWorld" false))

(fn ConstructionScript
  (Transformation|SetWorldScale3D (Variables|Debug|GetStaticMeshComponent) "0.100000,0.100000,0.100000"))