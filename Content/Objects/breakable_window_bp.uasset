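; Breakable window for VR that yields knife actors when struck by a motion controller.
; An overlap from a fast-moving BP_MotionController plays a glass-break sound and spawns a Knife_bp near the mesh with random rotation.
; A Hit flag and short delay debounce strikes while a counter tracks spawns.
; Once the spawn limit is reached, the next controller overlap at any speed destroys the window; the Break function is empty.
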(event Collision|EventActorBeginOverlap
  (params (OtherActor :type Actor%20Object%20Reference))
  (bind _staticmeshcomponent (Variables|Debug|GetStaticMeshComponent))
  (bind _returnvalue (Transformation|GetWorldTransform _staticmeshcomponent))
  (bind (_location _rotation _scale) (Math|Transform|BreakTransform _returnvalue))
  (bind (_x _y _z) (Math|Vector|BreakVector _location))
  (if (== (Utilities|GetClass OtherActor) "/Game/VirtualRealityBP/Blueprints/BP_MotionController.BP_MotionController_C")
    (if (< (Variables|Default|GetSpawned%20Knives) 5)
      (bind _asbp_motion_controller (Utilities|Casting|CastToBP_MotionController OtherActor))
      (if (and (> (Variables|/Game/VirtualRealityBP/Blueprints/BP_MotionController.BP_MotionController_C|GetSpeed _asbp_motion_controller) 5.0) (not (Variables|Default|Gethit)))
        (Audio|PlaySoundatLocation "/Game/Audio/glass_break.glass_break" (Transformation|GetWorldLocation (Variables|Debug|GetStaticMeshComponent)) "0, 0,0.000000" 1.0 0.5)
        (Game|SpawnActorfromClass "/Game/Objects/V4/knife_bp.knife_bp_C" (Math|Transform|MakeTransform (Math|Vector|MakeVector (+ _x 5.0) _y _z) (Math|Random|RandomRotator false) _scale) "Undefined" 0 0)
        (Variables|Default|Sethit true)
        (Utilities|FlowControl|Delay 0.5)
        (Variables|Default|Sethit false)
        (Math|Integer|IncrementInt (Variables|Default|GetSpawned%20Knives)))
      (else
        (Actor|DestroyActor)))))

(fn ConstructionScript)

(fn Break)