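; Short-lived fire object that can be picked up and dropped, and destroys itself after TimeBeforeFireRunsOut.
; Pickup disables mesh physics and attaches the root to the given component, while Drop restores physics and detaches.
; The construction script shrinks the mesh to a tenth scale.
; A Break Table function, not called within this Blueprint, hides the mesh, spawns four table pegs and a tabletop, then destroys the actor.
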(event EventBeginPlay
  (Utilities|FlowControl|Delay (Variables|Default|GetTimeBeforeFireRunsOut))
  (Actor|DestroyActor))

(event Collision|EventActorBeginOverlap
  (params (OtherActor :type Actor%20Object%20Reference)))

(event EventTick
  (params (DeltaSeconds :type Float%20%28single-precision%29)))

(event EventDrop
  (Physics|SetSimulatePhysics (Variables|Debug|GetStaticMeshComponent) true)
  (Transformation|DetachFromActor "KeepWorld" "KeepWorld" "KeepWorld"))

(event EventPickup
  (params (AttachTo :type Scene%20Component%20Object%20Reference))
  (Physics|SetSimulatePhysics (Variables|Debug|GetStaticMeshComponent) false)
  (Transformation|AttachComponentToComponent (VehicleSound|GetRootComponent) AttachTo "None" "KeepWorld" "KeepWorld" "KeepWorld" false))

(fn ConstructionScript
  (Transformation|SetWorldScale3D (Variables|Debug|GetStaticMeshComponent) "0.100000,0.100000,0.100000"))

(fn BreakTable
  (bind _staticmeshcomponent (Variables|Debug|GetStaticMeshComponent))
  (bind _returnvalue (Transformation|GetWorldLocation _staticmeshcomponent))
  (bind _returnvalue_2 (Transformation|GetWorldScale _staticmeshcomponent))
  (bind _returnvalue_3 (Math|Transform|MakeTransform _returnvalue "0, 0, 0" _returnvalue_2))
  (Development|SetHiddeninGame _staticmeshcomponent true false)
  (Game|SpawnActorfromClass "/Game/Objects/tablepeg_bp.tablepeg_bp_C" _returnvalue_3 "Undefined" 0 0)
  (Game|SpawnActorfromClass "/Game/Objects/tablepeg_bp.tablepeg_bp_C" _returnvalue_3 "Undefined" 0 0)
  (Game|SpawnActorfromClass "/Game/Objects/tablepeg_bp.tablepeg_bp_C" _returnvalue_3 "Undefined" 0 0)
  (Game|SpawnActorfromClass "/Game/Objects/tablepeg_bp.tablepeg_bp_C" _returnvalue_3 "Undefined" 0 0)
  (Game|SpawnActorfromClass "/Game/Objects/tabletop_bp.tabletop_bp_C" _returnvalue_3 "Undefined" 0 0)
  (Actor|DestroyActor))