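; A shovel prop that can be picked up and dropped, and breaks into its component objects when it hits something fast enough.
; Pickup turns off physics and attaches it to the given component, and Drop restores physics and detaches it.
; A hit with mesh velocity above BreakSpeed spawns a vent plus either a pipe or a table peg, chosen by IsPipe, then destroys the shovel.
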(event OnComponentHit(StaticMeshComponent)
  (params (HitComponent :type Primitive%20Component%20Object%20Reference) (OtherActor :type Actor%20Object%20Reference) (OtherComp :type Primitive%20Component%20Object%20Reference) (NormalImpulse :type Vector :default "0, 0, 0") (Hit :type Hit%20Result%20Structure%20%28by%20ref%29))
  (if (> (Math|Vector|VectorLength (Transformation|GetComponentVelocity (Variables|Debug|GetStaticMeshComponent))) (Variables|Default|GetBreak%20Speed))
    ;[1 1 1] NOT TESTED
    (CallFunction|BreakShovel)))

(event EventDrop
  (Physics|SetSimulatePhysics (Variables|Debug|GetStaticMeshComponent) true)
  (Transformation|DetachFromActor "KeepWorld" "KeepWorld" "KeepWorld"))

(event EventPickup
  (params (AttachTo :type Scene%20Component%20Object%20Reference))
  (Physics|SetSimulatePhysics (Variables|Debug|GetStaticMeshComponent) false)
  (Transformation|AttachComponentToComponent (VehicleSound|GetRootComponent) AttachTo "None" "KeepWorld" "KeepWorld" "KeepWorld" false))

(fn ConstructionScript)

(fn BreakShovel
  (bind _staticmeshcomponent (Variables|Debug|GetStaticMeshComponent))
  (bind _returnvalue (Transformation|GetWorldLocation _staticmeshcomponent))
  (bind _returnvalue_2 (Transformation|GetWorldScale _staticmeshcomponent))
  (bind _returnvalue_3 (Math|Transform|MakeTransform _returnvalue "0, 0, 0" _returnvalue_2))
  (Development|SetHiddeninGame _staticmeshcomponent true false)
  (Game|SpawnActorfromClass "/Game/Objects/V4/vent_bp.vent_bp_C" _returnvalue_3 "Undefined" 0 0)
  (if (Variables|Default|GetisPipe)
    (Game|SpawnActorfromClass "/Game/Objects/V4/pipe_bp.pipe_bp_C" _returnvalue_3 "Undefined" 0 0)
    (else
      (Game|SpawnActorfromClass "/Game/Objects/tablepeg_bp.tablepeg_bp_C" _returnvalue_3 "Undefined" 0 0)))
  (Actor|DestroyActor))