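; Knife prop Blueprint that can be picked up and dropped, and makes a sound on impact.
; Pickup disables mesh physics and attaches the root to the supplied component in world space, while Drop re-enables physics and detaches it.
; Hit plays the drop sound above a speed threshold, scaling volume with velocity and using a half-second flag cooldown to limit repeats.
; The construction script sets a fixed mesh scale.
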(event EventBeginPlay)

(event Collision|EventActorBeginOverlap
  (params (OtherActor :type Actor%20Object%20Reference)))

(event EventTick
  (params (DeltaSeconds :type Float%20%28single-precision%29)))

(event EventDrop
  (Physics|SetSimulatePhysics (Variables|Debug|GetStaticMeshComponent) true)
  (Transformation|DetachFromActor "KeepWorld" "KeepWorld" "KeepWorld"))

(event EventPickup
  (params (AttachTo :type Scene%20Component%20Object%20Reference))
  (Physics|SetSimulatePhysics (Variables|Debug|GetStaticMeshComponent) false)
  (Transformation|AttachComponentToComponent (VehicleSound|GetRootComponent) AttachTo "None" "KeepWorld" "KeepWorld" "KeepWorld" false))

(event Collision|EventHit
  (params (MyComp :type Primitive%20Component%20Object%20Reference) (Other :type Actor%20Object%20Reference) (OtherComp :type Primitive%20Component%20Object%20Reference) (bSelfMoved :type Boolean) (HitLocation :type Vector) (HitNormal :type Vector :default "0, 0, 0") (NormalImpulse :type Vector :default "0, 0, 0") (Hit :type Hit%20Result%20Structure%20%28by%20ref%29))
  (bind _staticmeshcomponent (Variables|Debug|GetStaticMeshComponent))
  (bind _returnvalue (Transformation|GetComponentVelocity _staticmeshcomponent))
  (bind _returnvalue_2 (Math|Vector|VectorLength _returnvalue))
  (if (and (> _returnvalue_2 5e+01) (not (Variables|Default|Gethit)))
    (Audio|PlaySoundatLocation "/Game/Audio/drop.drop" HitLocation "0, 0, 0" (/ _returnvalue_2 5e+01) 5e+01)
    (Variables|Default|Sethit true)
    (Utilities|FlowControl|Delay 0.5)
    (Variables|Default|Sethit false)))

(fn ConstructionScript
  (Transformation|SetWorldScale3D (Variables|Debug|GetStaticMeshComponent) "0.100000,0.250000,0.250000"))