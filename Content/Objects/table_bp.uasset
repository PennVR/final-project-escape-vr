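; Physics table prop that can be picked up, dropped and smashed.
; Pickup turns off physics and attaches the root to the given component, and Drop restores physics and detaches it.
; A mesh hit while moving faster than BreakSpeed calls BreakTable.
; BreakTable hides the mesh, spawns separate leg and top piece actors at its location with default rotation, then destroys the table.
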(event OnComponentHit(StaticMeshComponent)
  (params (HitComponent :type Primitive%20Component%20Object%20Reference) (OtherActor :type Actor%20Object%20Reference) (OtherComp :type Primitive%20Component%20Object%20Reference) (NormalImpulse :type Vector :default "0, 0, 0") (Hit :type Hit%20Result%20Structure%20%28by%20ref%29))
  (if (> (Math|Vector|VectorLength (Transformation|GetComponentVelocity (Variables|Debug|GetStaticMeshComponent))) (Variables|Default|GetBreak%20Speed))
    (CallFunction|BreakTable)))

(event EventBeginPlay)

(event Collision|EventActorBeginOverlap
  (params (OtherActor :type Actor%20Object%20Reference)))

(event EventTick
  (params (DeltaSeconds :type Float%20%28single-precision%29)))

(event EventDrop
  (Physics|SetSimulatePhysics (Variables|Debug|GetStaticMeshComponent) true)
  (Transformation|DetachFromActor "KeepWorld" "KeepWorld" "KeepWorld"))

(event EventPickup
  (params (AttachTo :type Scene%20Component%20Object%20Reference))
  (Physics|SetSimulatePhysics (Variables|Debug|GetStaticMeshComponent) false)
  (Transformation|AttachComponentToComponent (VehicleSound|GetRootComponent) AttachTo "None" "KeepWorld" "KeepWorld" "KeepWorld" false))

(fn ConstructionScript)

(fn BreakTable
  (bind _staticmeshcomponent (Variables|Debug|GetStaticMeshComponent))
  (bind _returnvalue (Transformation|GetWorldLocation _staticmeshcomponent))
  (bind _returnvalue_2 (Math|Transform|MakeTransform _returnvalue))
  (Development|SetHiddeninGame _staticmeshcomponent true false)
  (Game|SpawnActorfromClass "/Game/Objects/tablepeg_bp.tablepeg_bp_C" _returnvalue_2 "Undefined" 0 0)
  (Game|SpawnActorfromClass "/Game/Objects/tablepeg_bp.tablepeg_bp_C" _returnvalue_2 "Undefined" 0 0)
  (Game|SpawnActorfromClass "/Game/Objects/tablepeg_bp.tablepeg_bp_C" _returnvalue_2 "Undefined" 0 0)
  (Game|SpawnActorfromClass "/Game/Objects/tablepeg_bp.tablepeg_bp_C" _returnvalue_2 "Undefined" 0 0)
  (Game|SpawnActorfromClass "/Game/Objects/tabletop_bp.tabletop_bp_C" _returnvalue_2 "Undefined" 0 0)
  (Actor|DestroyActor))